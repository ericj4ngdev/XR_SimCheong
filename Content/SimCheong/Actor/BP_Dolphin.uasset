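; Dolphin actor that travels along a spline path placed in the level, starting at BeginPlay.
; It finds the SplinePath_Dolphin actor, then plays the MoveDolphin timeline at a rate of 1/TimetoComplete to control travel time.
; Each update maps the timeline alpha to distance along the spline and sets the actor's transform, using world-space location but local-space spline rotation.
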(event `self.ReceiveBeginPlay`
  (bind _returnvalue (`GameplayStatics.GetActorOfClass` "/Game/SimCheong/Actor/SplinePath_Dolphin.SplinePath_Dolphin_C"))
  (set `self.SplineRef_Dolphin` _returnvalue)
  (`self.Move Object`))

(event `Move Object`
  (bind _spline (`/Game/SimCheong/Actor/SplinePath_Dolphin.Spline` (`self.SplineRef_Dolphin`)))
  (`TimelineComponent.SetPlayRate` (`self.MoveDolphin`) (/ 1.0 (`self.TimetoComplete`))) ; 재생속도 설정
  (bind (_direction _movetrack) (`Timeline|MoveDolphin`) ; 더블 클릭시 속도 그래프 조정
    (:`Update`
      (bind _returnvalue (`KismetMathLibrary.Lerp` 0.0 (`SplineComponent.GetSplineLength` (`/Game/SimCheong/Actor/SplinePath_Dolphin.Spline` (`self.SplineRef_Dolphin`))) _movetrack))
      (`self.K2_SetActorTransform` (`KismetMathLibrary.MakeTransform` (`SplineComponent.GetLocationAtDistanceAlongSpline` _spline _returnvalue "World") (`SplineComponent.GetRotationAtDistanceAlongSpline` _spline _returnvalue "Local"))))))

(fn `UserConstructionScript`)