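; BP_Turtle is an actor that travels along a spline path in the level.
; On BeginPlay it finds the SplinePath_turtle actor and plays a timeline at a rate of one over TimetoComplete.
; Each update maps the timeline's MoveTrack curve to a distance along the spline, so the curve shapes the speed.
; The actor takes its location from the spline in world space and its rotation in local space.
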(event `self.ReceiveBeginPlay`
  (bind _returnvalue (`GameplayStatics.GetActorOfClass` "/Game/SimCheong/Actor/SplinePath_turtle.SplinePath_turtle_C"))
  (set `self.SplineRef` _returnvalue)
  (`self.Move Object`))

(event `Move Object`
  (bind _spline (`/Game/SimCheong/Actor/SplinePath_turtle.Spline` (`self.SplineRef`)))
  (`TimelineComponent.SetPlayRate` (`self.Move Obeject T`) (/ 1.0 (`self.TimetoComplete`))) ; 재생속도 설정
  (bind (_direction _movetrack) (`Timeline|Move Obeject T`) ; 더블 클릭시 속도 그래프 조정
    (:`Update`
      (bind _returnvalue (`KismetMathLibrary.Lerp` 0.0 (`SplineComponent.GetSplineLength` (`/Game/SimCheong/Actor/SplinePath_turtle.Spline` (`self.SplineRef`))) _movetrack))
      (`self.K2_SetActorTransform` (`KismetMathLibrary.MakeTransform` (`SplineComponent.GetLocationAtDistanceAlongSpline` _spline _returnvalue "World") (`SplineComponent.GetRotationAtDistanceAlongSpline` _spline _returnvalue "Local"))))))

(fn `UserConstructionScript`)