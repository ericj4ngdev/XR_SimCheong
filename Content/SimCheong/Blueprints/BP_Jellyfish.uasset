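; BP_Jellyfish is a placeable jellyfish actor with a mesh and point light that bobs up and down around its spawn position.
; The construction script uses Size to scale both the mesh and the light's attenuation radius.
; BeginPlay stores the start location and randomises phase, speed and amplitude, so instances move out of sync.
; Tick accumulates time and sets the actor's height with a sine wave.
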(event `self.ReceiveBeginPlay`
  (set `self.InitialLocation` (`self.K2_GetActorLocation`))
  (set `self.Time` (/ (`KismetMathLibrary.RandomFloatInRange` -180.0 180.0) (`self.Speed`)))
  (set `self.Speed` (* (`self.Speed`) (`KismetMathLibrary.RandomFloatInRange` 0.8 1.2)))
  (set `self.Pitch` (* (`self.Pitch`) (`KismetMathLibrary.RandomFloatInRange` 0.8 1.2))))

(event `self.ReceiveTick`
  (params (DeltaSeconds :type "Float (single-precision)"))
  (set `self.Time` (+ DeltaSeconds (`self.Time`)))
  (`self.K2_SetActorLocation` (+ (`self.InitialLocation`) (`KismetMathLibrary.MakeVector` 0.0 0.0 (* (`KismetMathLibrary.DegSin` (* (`self.Time`) (`self.Speed`))) (`self.Pitch`))))))

(fn `UserConstructionScript`
  (bind _size (`self.Size`))
  (`SceneComponent.SetWorldScale3D` (`self.StaticMesh`) (`KismetMathLibrary.MakeVector` _size _size _size))
  (`LocalLightComponent.SetAttenuationRadius` (`self.PointLight`) (* (`self.Size`) 500.0)))